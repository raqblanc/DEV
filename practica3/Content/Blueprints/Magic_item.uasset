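; Magic item pickup Blueprint that raises the player's magic level when overlapped and then destroys itself.
; The overlap event casts the game instance to TestGameInstance and calls UpdateMagicLevel with an amount chosen by the ItemType enum (Lightning, Falme or SnowFlake).
; The construction script also selects the static mesh from ItemType, with no mesh assigned for Falme.
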(event `self.Overlap.OnComponentBeginOverlap`
  (params (OverlappedComponent :type "PrimitiveComponent Object Reference") (OtherActor :type "Actor Object Reference") (OtherComp :type "PrimitiveComponent Object Reference") (OtherBodyIndex :type Integer) (bFromSweep :type Boolean) (SweepResult :type "HitResult Structure (by ref)"))
  (bind _astest_game_instance (cast `/Game/Blueprints/TestGameInstance` (`GameplayStatics.GetGameInstance`)))
  (`/Game/Blueprints/TestGameInstance.UpdateMagicLevel` _astest_game_instance (select `/Game/Blueprints/EItemType` (`self.ItemType`) :`NewEnumerator0` 0.2 :`NewEnumerator1` 0.1 :`NewEnumerator2` 0.15 :!type "Float (single-precision)"))
  (`self.K2_DestroyActor`))

(fn `UserConstructionScript`
  (`StaticMeshComponent.SetStaticMesh` (`self.MagicItem`) (select `/Game/Blueprints/EItemType` (`self.ItemType`) :`NewEnumerator0` "/Game/ContenidoDescargado/EF_Edie/Meshes/Armchair_b.Armchair_b" :`NewEnumerator2` "/Game/ContenidoDescargado/EF_Edie/Meshes/birdcage_c.birdcage_c" :!type "StaticMesh Object Reference")))