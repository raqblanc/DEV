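; Neighbour NPC character that shows a press-S talk prompt when the player overlaps its collision box and can spawn a key.
; Overlap events manage the GameInstance's prompt and hidden dialog widgets; Speak hides the prompt.
; SpawnKey creates one BP_Key while overlapping, at random navmesh coordinates shifted by the box extent, intended to land outside it, and slightly raised.
; Stop and Start functions toggle its walk speed.
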(event `self.CollisionDistance.OnComponentBeginOverlap`
  (params (OverlappedComponent :type "PrimitiveComponent Object Reference") (OtherActor :type "Actor Object Reference") (OtherComp :type "PrimitiveComponent Object Reference") (OtherBodyIndex :type Integer) (bFromSweep :type Boolean) (SweepResult :type "HitResult Structure (by ref)"))
  ;[1 1 1] Cuando entra en el radio del vecino, aparece el mensaje de pulsar S para hablar
  (cast `/Game/TopDownBP/Blueprints/TopDownCharacter` OtherActor)
  (set `self.Overlapping` true)
  (bind _astest_game_instance (cast `/Game/Blueprints/TestGameInstance` (`GameplayStatics.GetGameInstance`)))
  (bind _pressswidget (`/Game/Blueprints/TestGameInstance.pressSwidget` _astest_game_instance))
  (if (`Widget.IsInViewport` _pressswidget)
    (`Widget.SetVisibility` _pressswidget "Visible")
    (else
      (`UserWidget.AddToViewport` _pressswidget 0)))
  (bind _dialogbox (`/Game/Blueprints/TestGameInstance.DialogBox` _astest_game_instance))
  (if (not (`Widget.IsInViewport` _dialogbox))
    (`UserWidget.AddToViewport` _dialogbox 0)
    (`Widget.SetVisibility` _dialogbox "Hidden")))

(event `self.CollisionDistance.OnComponentEndOverlap`
  (params (OverlappedComponent :type "PrimitiveComponent Object Reference") (OtherActor :type "Actor Object Reference") (OtherComp :type "PrimitiveComponent Object Reference") (OtherBodyIndex :type Integer))
  ;[1 1 1] Cuando entra en el radio del vecino, aparece el mensaje de pulsar S para hablar
  (cast `/Game/TopDownBP/Blueprints/TopDownCharacter` OtherActor)
  (`Widget.SetVisibility` (`/Game/Blueprints/TestGameInstance.pressSwidget` (stale `self.CollisionDistance.OnComponentBeginOverlap` _astest_game_instance)) "Hidden")
  (set `self.Overlapping` false))

(fn `calculatePoint`
  (params (CollisionPoint :type "Float (double-precision)") (RandomPoint :type "Float (double-precision)"))
  (returns (SpawnPoint :type "Float (double-precision)"))
  ;[1 1 1] Collision point es el tamaño de la caja de colisión. Esta función calcula un punto que salga fuera de la caja (para que no haya posibilidad de que el player coja el objeto sin tener que desplazarse). Vale para X y para Y.
  (if (< RandomPoint 0.0)
    (return (- RandomPoint CollisionPoint))
    (else
      (return (+ CollisionPoint RandomPoint)))))

(fn `getSpawnTransform`
  (returns (transform :type "Transform Structure"))
  (locals (X :type "Float (double-precision)" :default 0.0) (Y :type "Float (double-precision)"))
  (bind _spawnpoint (`self.calculatePoint` (.x (`BoxComponent.GetScaledBoxExtent` (`self.CollisionDistance`))) (.x (`NavigationSystemV1.K2_GetRandomLocationInNavigableRadius` (.location (`self.GetTransform`)) 500.0 null "/Script/NavigationSystem.RecastFilter_UseDefaultArea"))))
  (bind _output_get (set `local.X` _spawnpoint))
  (bind _spawnpoint_2 (`self.calculatePoint` (.y (`BoxComponent.GetScaledBoxExtent` (`self.CollisionDistance`))) (.y (`NavigationSystemV1.K2_GetRandomLocationInNavigableRadius` (.location (`self.GetTransform`)) 500.0 null "/Script/NavigationSystem.RecastFilter_UseDefaultArea"))))
  (bind _output_get_2 (set `local.Y` _spawnpoint_2))
  (return (`KismetMathLibrary.MakeTransform` (`KismetMathLibrary.MakeVector` _output_get _output_get_2 (+ (.z (`NavigationSystemV1.K2_GetRandomLocationInNavigableRadius` (.location (`self.GetTransform`)) 500.0 null "/Script/NavigationSystem.RecastFilter_UseDefaultArea")) 50.0)) (.rotation (`self.GetTransform`)) (.scale (`self.GetTransform`)))))

(fn `SpawnKey`
  ;[1 1 1] Spawnea al objeto llave
  (if (and (not (`self.Spawned`)) (`self.Overlapping`))
    (set `self.Spawned` true)
    (bind _transform (`self.getSpawnTransform`))
    (bind _returnvalue (`|SpawnActorFromClass` "/Game/Blueprints/BP_Key.BP_Key_C" _transform "AdjustIfPossibleButAlwaysSpawn" "OverrideRootScale" null null))
    (`/Game/Blueprints/BP_Key.setMaterial` _returnvalue (`self.KeyType`))))

(fn `Speak`
  (bind _astest_game_instance (cast `/Game/Blueprints/TestGameInstance` (`GameplayStatics.GetGameInstance`)))
  (if (`self.Overlapping`)
    (`Widget.SetVisibility` (`/Game/Blueprints/TestGameInstance.pressSwidget` _astest_game_instance) "Hidden")))

(fn `StartNeighbour`
  (set `CharacterMovementComponent.MaxWalkSpeed` 100.0 (`self.CharacterMovement`)))

(fn `StopNeighbour`
  (set `CharacterMovementComponent.MaxWalkSpeed` 0.0 (`self.CharacterMovement`)))

(fn `UserConstructionScript`)