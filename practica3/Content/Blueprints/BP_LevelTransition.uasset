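; BP_LevelTransition is a level exit that opens a named level when its Overlap component is overlapped and its requirements are met.
; BeginPlay caches the TestGameInstance, which supplies the key count and magic level.
; The overlap requires exactly one key of the required type and enough magic, without checking which actor entered.
; The construction script derives the magic threshold from the key type, currently identical for every floor.
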(event `self.ReceiveBeginPlay`
  (bind _astest_game_instance (cast `/Game/Blueprints/TestGameInstance` (`GameplayStatics.GetGameInstance`)))
  (set `self.GameInstance` _astest_game_instance))

(event `self.Overlap.OnComponentBeginOverlap`
  (params (OverlappedComponent :type "PrimitiveComponent Object Reference") (OtherActor :type "Actor Object Reference") (OtherComp :type "PrimitiveComponent Object Reference") (OtherBodyIndex :type Integer) (bFromSweep :type Boolean) (SweepResult :type "HitResult Structure (by ref)"))
  (bind _gameinstance (`self.GameInstance`))
  (bind _value (`/Game/Blueprints/TestGameInstance.GetNKeys` _gameinstance (`self.RequireKeyType`)))
  (if (and (== _value 1) (<= (`self.required_magic_level`) (`/Game/Blueprints/TestGameInstance.Magic_Level` _gameinstance)))
    (`GameplayStatics.OpenLevel` (`self.LevelName`))))

(fn `UserConstructionScript`
  (set `self.required_magic_level` (select `/Game/Blueprints/EKeyType` (`self.RequireKeyType`) :`NewEnumerator1` 0.1 :`NewEnumerator2` 0.1 :`NewEnumerator3` 0.1 :!type "Float (single-precision)")))