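; Neighbour actor that shows a "press S to talk" prompt when the TopDownCharacter enters its box trigger.
; The prompt widget lives on TestGameInstance and is added to the viewport or made visible on overlap, then hidden on exit.
; Input is enabled at BeginPlay, so S hides the prompt and spawns an actor at the neighbour's transform, with no in-range check.
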(event `self.ReceiveBeginPlay`
  ;[1 1 1] Cuando entra en el radio del vecino, aparece el mensaje de pulsar S para hablar
  (`self.EnableInput` (`GameplayStatics.GetPlayerController` 0)))

(event `Key|S`
  (params (Key :type "Key Structure"))
  (:`Pressed`
    (`Widget.SetVisibility` (`/Game/Blueprints/TestGameInstance.pressSwidget` (stale `self.Box.OnComponentBeginOverlap` _astest_game_instance)) "Hidden")
    (`|SpawnActorFromClass` "/Game/Blueprints/BP_Key.BP_Key_C" (`self.GetTransform`) "AdjustIfPossibleButAlwaysSpawn" "OverrideRootScale" null null)))

(event `self.Box.OnComponentBeginOverlap`
  (params (OverlappedComponent :type "PrimitiveComponent Object Reference") (OtherActor :type "Actor Object Reference") (OtherComp :type "PrimitiveComponent Object Reference") (OtherBodyIndex :type Integer) (bFromSweep :type Boolean) (SweepResult :type "HitResult Structure (by ref)"))
  ;[1 1 1] Cuando entra en el radio del vecino, aparece el mensaje de pulsar S para hablar
  (cast `/Game/TopDownBP/Blueprints/TopDownCharacter` OtherActor)
  (bind _astest_game_instance (cast `/Game/Blueprints/TestGameInstance` (`GameplayStatics.GetGameInstance`)))
  (bind _pressswidget (`/Game/Blueprints/TestGameInstance.pressSwidget` _astest_game_instance))
  (if (`Widget.IsInViewport` _pressswidget)
    (`Widget.SetVisibility` _pressswidget "Visible")
    (else
      (`UserWidget.AddToViewport` _pressswidget 0))))

(event `self.Box.OnComponentEndOverlap`
  (params (OverlappedComponent :type "PrimitiveComponent Object Reference") (OtherActor :type "Actor Object Reference") (OtherComp :type "PrimitiveComponent Object Reference") (OtherBodyIndex :type Integer))
  ;[1 1 1] Cuando entra en el radio del vecino, aparece el mensaje de pulsar S para hablar
  (`Widget.SetVisibility` (`/Game/Blueprints/TestGameInstance.pressSwidget` (stale `self.Box.OnComponentBeginOverlap` _astest_game_instance)) "Hidden"))

(fn `UserConstructionScript`)