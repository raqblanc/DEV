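; PilaAmarilla is a yellow battery pickup that grants the first-person character three powerful jumps.
; On BeginPlay it caches MiGameInstance, which holds the shared jump state.
; When the character overlaps its Cube, it flags yellow as active only if the jump count is zero, adds to that count, then destroys itself.
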(event `self.ReceiveBeginPlay`
  ;[1 1 1] Coger las variable globales
  (bind _asmi_game_instance (cast `/Game/Blueprints/MiGameInstance` (`GameplayStatics.GetGameInstance`))))

(event `self.Cube.OnComponentBeginOverlap`
  (params (OverlappedComponent :type "PrimitiveComponent Object Reference") (OtherActor :type "Actor Object Reference") (OtherComp :type "PrimitiveComponent Object Reference") (OtherBodyIndex :type Integer) (bFromSweep :type Boolean) (SweepResult :type "HitResult Structure (by ref)"))
  (cast `/Game/Blueprints/FirstPersonCharacter` OtherActor)
  (bind _n_saltos (`/Game/Blueprints/MiGameInstance.n_saltos` (stale `self.ReceiveBeginPlay` _asmi_game_instance)))
  ;[1 1 1] Si es la primera pila (n_saltos == 0) se activa
  (if (== 0 _n_saltos)
    (set `/Game/Blueprints/MiGameInstance.amarilla_activa` true (stale `self.ReceiveBeginPlay` _asmi_game_instance)))
  ;[1 1 1] Se suman 3 saltos potentes
  (set `/Game/Blueprints/MiGameInstance.n_saltos` (+ _n_saltos 3) (stale `self.ReceiveBeginPlay` _asmi_game_instance))
  (`self.K2_DestroyActor`))

(fn `UserConstructionScript`)