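; Cabina is a shootable booth that spawns Enemigo AI pawns until it is knocked out and becomes electrified.
; Tick uses Delays to pace an initial wave, then refills when the GameInstance's shared enemy count runs low.
; Normal and special projectiles subtract Vida; exactly zero sets Electrico, stopping spawns and decrementing the active-booth count.
; Sparks show when Electrico and global Electricidad are both true, and EstaElectrificada exposes the booth's state.
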(event `self.ReceiveBeginPlay`
  ;[1 1 1] Coger las variable globales
  (bind _asmi_game_instance (cast `/Game/Blueprints/MiGameInstance` (`GameplayStatics.GetGameInstance`)))
  (set `self.ginstance` _asmi_game_instance)
  (`SceneComponent.SetVisibility` (`self.P_Sparks1`) false true))

(event `self.ReceiveHit`
  (params (MyComp :type "PrimitiveComponent Object Reference") (Other :type "Actor Object Reference") (OtherComp :type "PrimitiveComponent Object Reference") (bSelfMoved :type Boolean) (HitLocation :type "Vector Structure") (HitNormal :type "Vector Structure") (NormalImpulse :type "Vector Structure") (Hit :type "HitResult Structure (by ref)"))
  (bind _vida (`self.vida`))
  (bind _ginstance (`self.ginstance`))
  ;[1 1 1] Cuando se dispara a la cabina se le quita vida y si se queda sin vida salta el evento para cambiar la electricidad
  (cast `/Game/Blueprints/Proyectil/Proyectil` Other
    (:`then`
      (set `self.vida` (- _vida 1)))
    (:`CastFailed`
      (cast `/Game/Blueprints/Proyectil/ProyectilEspecial` Other)
      (set `self.vida` (- _vida 3))))
  (if (== _vida 0)
    (set `self.electrico` true)
    (set `/Game/Blueprints/MiGameInstance.num_cabinas_activas` (- (`/Game/Blueprints/MiGameInstance.num_cabinas_activas` _ginstance) 1) _ginstance)
    (`self.CambioElectricidadCabina`)))

(event `SpawnEnemigo`
  (bind _ginstance (`self.ginstance`))
  ;[1 1 1] Spawnear 1 enemigo
  (if (not (`self.electrico`))
    (bind _returnvalue (`AIBlueprintHelperLibrary.SpawnAIFromClass` "/Game/Blueprints/IA/Enemigo.Enemigo_C" "/Game/Blueprints/IA/BT_Enemigo.BT_Enemigo" (`KismetMathLibrary.MakeVector` (- (.x (`self.K2_GetActorLocation`)) 300.0) (.y (`self.K2_GetActorLocation`)) (.z (`self.K2_GetActorLocation`))) (struct) false null))
    (cast `/Game/Blueprints/IA/Enemigo` _returnvalue)
    (set `/Game/Blueprints/MiGameInstance.num_enemigos` (+ (`/Game/Blueprints/MiGameInstance.num_enemigos` _ginstance) 1) _ginstance)))

(event `CambioElectricidadCabina`
  ;[1 1 1] Electrificar la cabina
  (`SceneComponent.SetVisibility` (`self.P_Sparks1`) (and (`self.electrico`) (`/Game/Blueprints/MiGameInstance.electricidad` (`self.ginstance`))) true))

(event `self.ReceiveTick`
  (params (DeltaSeconds :type "Float (single-precision)"))
  ;[1 1 1] Spawnea enemigos cada 2s cuando se inicia o se resetea el juego
  (if (`self.primer_spawn`)
    (`KismetSystemLibrary.Delay` 2.0)
    (if (< (`/Game/Blueprints/MiGameInstance.num_enemigos` (`self.ginstance`)) 9)
      (`self.SpawnEnemigo`)
      (else
        (set `self.primer_spawn` false)))
    (else
      ;[1 1 1] Spawnear enemigos cuando hay pocos
      (if (< (`/Game/Blueprints/MiGameInstance.num_enemigos` (`self.ginstance`)) 5)
        (`self.SpawnEnemigo`)
        (`KismetSystemLibrary.Delay` 2.0)
        (`self.SpawnEnemigo`)
        (`KismetSystemLibrary.Delay` 2.0)
        (`self.SpawnEnemigo`)
        (`KismetSystemLibrary.Delay` 2.0)
        (`self.SpawnEnemigo`)
        (`KismetSystemLibrary.Delay` 2.0)))))

(fn `Esta Electrificada`
  (returns (electrificada :type Boolean))
  (return (`self.electrico`)))

(fn `UserConstructionScript`)