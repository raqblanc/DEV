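; BP_magic_item is a magic pickup actor in one of three types: lightning, flame or snowflake.
; The construction script selects the MagicItem static mesh from ItemType.
; When TopDownCharacter overlaps it, it registers the item in TestGameInstance and updates the magic level with that type's value stored there.
; It then plays a teleport sound at its location and destroys itself.
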(event `self.Overlap.OnComponentBeginOverlap`
  (params (OverlappedComponent :type "PrimitiveComponent Object Reference") (OtherActor :type "Actor Object Reference") (OtherComp :type "PrimitiveComponent Object Reference") (OtherBodyIndex :type Integer) (bFromSweep :type Boolean) (SweepResult :type "HitResult Structure (by ref)"))
  (bind _itemtype (`self.ItemType`))
  ;[1 1 1] Si se hace overlap con la caja del objeto mágico, se añade al inventario un ítem de ese tipo, se aumenta la magia según el valor que sea y se reproduce el sonido de obtención de item. Al final se destruye el actor.
  (cast `/Game/TopDownBP/Blueprints/TopDownCharacter` OtherActor)
  (bind _astest_game_instance (cast `/Game/Blueprints/TestGameInstance` (`GameplayStatics.GetGameInstance`)))
  (`/Game/Blueprints/TestGameInstance.SetNItems` _astest_game_instance _itemtype)
  (`/Game/Blueprints/TestGameInstance.UpdateMagicLevel` _astest_game_instance (select `/Game/Blueprints/Enums/EItemType` _itemtype :`NewEnumerator0` (`/Game/Blueprints/TestGameInstance.LightningValue` _astest_game_instance) :`NewEnumerator1` (`/Game/Blueprints/TestGameInstance.FlameValue` _astest_game_instance) :`NewEnumerator2` (`/Game/Blueprints/TestGameInstance.IceValue` _astest_game_instance)))
  (`GameplayStatics.PlaySoundAtLocation` "/Game/TandP/Sound_Effects/S_Teleport.S_Teleport" (`self.K2_GetActorLocation`) (struct) 1.0 1.0 0.0 null null null)
  (`self.K2_DestroyActor`))

(fn `UserConstructionScript`
  (`StaticMeshComponent.SetStaticMesh` (`self.MagicItem`) (select `/Game/Blueprints/Enums/EItemType` (`self.ItemType`) :!type "StaticMesh Object Reference")))