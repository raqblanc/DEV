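; Game instance that holds the player's shared UI widgets, magic level and key counts across levels.
; On Init it creates the HUD, PressS prompt and DialogBox widgets and stores references without adding them to the viewport.
; Helper functions add to the magic level and increment or return key counts tracked separately for the basement, first floor and second floor.
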(event `self.ReceiveInit`
  (bind _returnvalue (`|CreateWidget` "/Game/Widgets/HUD.HUD_C"))
  (set `self.HUD Reference` _returnvalue)
  (bind _returnvalue_2 (`|CreateWidget` "/Game/Widgets/PressS.PressS_C"))
  (set `self.pressSwidget` _returnvalue_2)
  (bind _returnvalue_3 (`|CreateWidget` "/Game/Widgets/DialogBox.DialogBox_C"))
  (set `self.DialogBox` _returnvalue_3))

(fn `GetNKeys`
  (params (Type :type "/Game/Blueprints/EKeyType Enum" :default "NewEnumerator1"))
  (returns (Value :type Integer))
  (switch `/Game/Blueprints/EKeyType` Type
    (:`NewEnumerator1`
      (return (`self.n_basement`)))
    (:`NewEnumerator2`
      (return (`self.n_firstfloor`)))
    (:`NewEnumerator3`
      (return (`self.n_secondfloor`)))))

(fn `SetNKeys`
  (params (Type :type "/Game/Blueprints/EKeyType Enum" :default "NewEnumerator1"))
  (switch `/Game/Blueprints/EKeyType` Type
    (:`NewEnumerator1`
      (`/Engine/EditorBlueprintResources/StandardMacros.IncrementInt` (`self.n_basement`)))
    (:`NewEnumerator2`
      (`/Engine/EditorBlueprintResources/StandardMacros.IncrementInt` (`self.n_firstfloor`)))
    (:`NewEnumerator3`
      (`/Engine/EditorBlueprintResources/StandardMacros.IncrementInt` (`self.n_secondfloor`)))))

(fn `UpdateMagicLevel`
  (params (Value :type "Float (double-precision)"))
  (set `self.Magic_Level` (+ Value (`self.Magic_Level`))))