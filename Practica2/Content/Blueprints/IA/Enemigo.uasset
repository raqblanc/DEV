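; Enemy character that can be killed by electrified objects and knocks the first-person player away on contact.
; Hitting electrified furniture or an electrified Cabina while the game instance's electricity flag is on decrements the shared enemy count and destroys the enemy.
; Capsule overlap with the player launches both characters along the enemy's velocity, scaled more strongly for the enemy itself.
; A helper function sets its maximum walk speed.
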(event `self.ReceiveBeginPlay`
  ;[1 1 1] Coger las variables globales
  (bind _asmi_game_instance (cast `/Game/Blueprints/MiGameInstance` (`GameplayStatics.GetGameInstance`)))
  (set `self.ginstance` _asmi_game_instance))

(event `self.ReceiveHit`
  (params (MyComp :type "PrimitiveComponent Object Reference") (Other :type "Actor Object Reference") (OtherComp :type "PrimitiveComponent Object Reference") (bSelfMoved :type Boolean) (HitLocation :type "Vector Structure") (HitNormal :type "Vector Structure") (NormalImpulse :type "Vector Structure") (Hit :type "HitResult Structure (by ref)"))
  (bind _ginstance (`self.ginstance`))
  (bind _electricidad (`/Game/Blueprints/MiGameInstance.electricidad` (`self.ginstance`)))
  (cast `/Game/Blueprints/MobiliarioElectrificado` Other
    (:`then`
      (if _electricidad
        (set `/Game/Blueprints/MiGameInstance.num_enemigos` (- (`/Game/Blueprints/MiGameInstance.num_enemigos` _ginstance) 1) _ginstance :!label _label)
        (`self.K2_DestroyActor`)))
    (:`CastFailed`
      (bind _ascabina (cast `/Game/Blueprints/Cabina` Other))
      (bind _electrificada (`/Game/Blueprints/Cabina.Esta Electrificada` _ascabina))
      (if (and _electrificada _electricidad)
        (goto _label)))))

(event `self.CapsuleComponent.OnComponentBeginOverlap`
  (params (OverlappedComponent :type "PrimitiveComponent Object Reference") (OtherActor :type "Actor Object Reference") (OtherComp :type "PrimitiveComponent Object Reference") (OtherBodyIndex :type Integer) (bFromSweep :type Boolean) (SweepResult :type "HitResult Structure (by ref)"))
  (bind _returnvalue (`self.GetVelocity`))
  (bind _aspersonaje_primera_persona (cast `/Game/Blueprints/PersonajePrimeraPersona` OtherActor))
  (`self.LaunchCharacter` _aspersonaje_primera_persona (* _returnvalue 5) false false)
  (`self.LaunchCharacter` (* _returnvalue 10))
  (`KismetSystemLibrary.Delay` 2.0))

(fn `cambiarVelocidad`
  (params (NuevaVelocidad :type "Float (double-precision)"))
  (set `CharacterMovementComponent.MaxWalkSpeed` NuevaVelocidad (`self.CharacterMovement`)))

(fn `UserConstructionScript`)