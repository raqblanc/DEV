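; Baldosa is a floor tile actor that acts as a trigger switching electricity on or off when the first-person character steps on it.
; On BeginPlay it caches the MiGameInstance.
; When PersonajePrimeraPersona overlaps the Cube, it flips the game instance's global Electricidad flag.
; It then notifies every MobiliarioElectrificado and Cabina actor in the level to update their electrical state.
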(event `self.ReceiveBeginPlay`
  ;[1 1 1] Coger las variable globales
  (bind _asmi_game_instance (cast `/Game/Blueprints/MiGameInstance` (`GameplayStatics.GetGameInstance`))))

(event `self.Cube.OnComponentBeginOverlap`
  (params (OverlappedComponent :type "PrimitiveComponent Object Reference") (OtherActor :type "Actor Object Reference") (OtherComp :type "PrimitiveComponent Object Reference") (OtherBodyIndex :type Integer) (bFromSweep :type Boolean) (SweepResult :type "HitResult Structure (by ref)"))
  (cast `/Game/Blueprints/PersonajePrimeraPersona` OtherActor)
  (set `/Game/Blueprints/MiGameInstance.electricidad` (not (`/Game/Blueprints/MiGameInstance.electricidad` (stale `self.ReceiveBeginPlay` _asmi_game_instance))) (stale `self.ReceiveBeginPlay` _asmi_game_instance))
  (bind _outactors (`GameplayStatics.GetAllActorsOfClass` "/Game/Blueprints/Cabina.Cabina_C"))
  (bind _outactors_2 (`GameplayStatics.GetAllActorsOfClass` "/Game/Blueprints/MobiliarioElectrificado.MobiliarioElectrificado_C"))
  (for _array_element _outactors_2
    (`/Game/Blueprints/MobiliarioElectrificado.CambioElectricidadMobiliario` _array_element))
  (for _array_element_2 _outactors
    (`/Game/Blueprints/Cabina.CambioElectricidadCabina` _array_element_2)))

(fn `UserConstructionScript`)