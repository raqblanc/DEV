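; AI controller for a Neighbour NPC that runs BT_Neighbour on possess and also takes keyboard input from player 0.
; S shows the game instance's dialog box and, while Overlapping, clears the neighbour timer and sets the HasLineOfSight and Continue blackboard keys.
; Enter hides the dialog and clears Continue, which Tick also clears whenever Overlapping is false.
; The Overlapping flag and dialog widget are both read from TestGameInstance.
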(event `self.ReceiveTick`
  (params (DeltaSeconds :type "Float (single-precision)"))
  (bind _astest_game_instance (cast `/Game/Blueprints/TestGameInstance` (`GameplayStatics.GetGameInstance`)))
  (if (not (`/Game/Blueprints/TestGameInstance.Overlapping` _astest_game_instance))
    (`BlackboardComponent.SetValueAsBool` (`self.Blackboard`) (`self.Continue`) false)))

(event `self.ReceiveBeginPlay`
  (`self.EnableInput` (`GameplayStatics.GetPlayerController` 0)))

(event `Key|S`
  (params (Key :type "Key Structure"))
  (bind _blackboard (`self.Blackboard`))
  (:`Pressed`
    (bind _astest_game_instance (cast `/Game/Blueprints/TestGameInstance` (`GameplayStatics.GetGameInstance`)))
    (`UserWidget.AddToViewport` (`/Game/Blueprints/TestGameInstance.DialogBox` _astest_game_instance) 0)
    (if (`/Game/Blueprints/TestGameInstance.Overlapping` _astest_game_instance)
      (`KismetSystemLibrary.K2_ClearAndInvalidateTimerHandle` (`self.NeighboutTimer`))
      (`BlackboardComponent.SetValueAsBool` _blackboard (`self.HasLineOfSight`) true)
      (`BlackboardComponent.SetValueAsBool` _blackboard (`self.Continue`) true))))

(event `self.ReceivePossess`
  (params (PossessedPawn :type "Pawn Object Reference"))
  (`self.RunBehaviorTree` "/Game/Blueprints/Neighbour/IA/BT_Neighbour.BT_Neighbour"))

(event `Key|Enter`
  (params (Key :type "Key Structure"))
  (:`Pressed`
    (bind _astest_game_instance (cast `/Game/Blueprints/TestGameInstance` (`GameplayStatics.GetGameInstance`)))
    (`Widget.SetVisibility` (`/Game/Blueprints/TestGameInstance.DialogBox` _astest_game_instance) "Hidden")
    (`BlackboardComponent.SetValueAsBool` (`self.Blackboard`) (`self.Continue`) false)))

(fn `UserConstructionScript`)