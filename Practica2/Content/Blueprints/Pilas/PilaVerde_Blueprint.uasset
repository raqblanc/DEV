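; PilaVerde is a green battery pickup that temporarily doubles the player's walk speed for five seconds.
; BeginPlay caches the original and doubled MaxWalkSpeed, and a FirstPersonCharacter overlapping the Cube hides the pickup and applies the boost.
; After a Delay it restores the cached speed and destroys itself, so boosts don't stack but each battery runs its own timer.
; The construction script caches MiGameInstance, which is otherwise unused here.
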(event `self.ReceiveBeginPlay`
  (bind _maxwalkspeed (`CharacterMovementComponent.MaxWalkSpeed` (`Character.CharacterMovement` (`GameplayStatics.GetPlayerCharacter` 0))))
  (set `self.velocidad_original` _maxwalkspeed)
  (set `self.supervelocidad` (* 2 _maxwalkspeed)))

(event `self.Cube.OnComponentBeginOverlap`
  (params (OverlappedComponent :type "PrimitiveComponent Object Reference") (OtherActor :type "Actor Object Reference") (OtherComp :type "PrimitiveComponent Object Reference") (OtherBodyIndex :type Integer) (bFromSweep :type Boolean) (SweepResult :type "HitResult Structure (by ref)"))
  (bind _charactermovement (`Character.CharacterMovement` (`GameplayStatics.GetPlayerCharacter` 0)))
  ;[1 1 1] Cuando el personaje se solapa con la pila se aumenta la velocidad durante 5 segundos. Si se coge más de una pila, se resetea el tiempo a 5s (no se vuelve a aumentar la velocidad)
  (cast `/Game/Blueprints/FirstPersonCharacter` OtherActor)
  (`SceneComponent.SetVisibility` (`self.DefaultSceneRoot`) false true)
  (set `CharacterMovementComponent.MaxWalkSpeed` (`self.supervelocidad`) _charactermovement)
  (`KismetSystemLibrary.Delay` 5.0)
  (set `CharacterMovementComponent.MaxWalkSpeed` (`self.velocidad_original`) _charactermovement)
  (`self.K2_DestroyActor`))

(fn `UserConstructionScript`
  ;[1 1 1] Coger las variable globales
  (bind _asmi_game_instance (cast `/Game/Blueprints/MiGameInstance` (`GameplayStatics.GetGameInstance`)))
  (set `self.ginstance` _asmi_game_instance))