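; Magic creature NPC that talks to the top-down character and hands over magic items.
; Its collision box registers the creature in TestGameInstance and toggles the press-S prompt, also closing the dialog box on exit.
; GetText, NextText and ReloadText step through the dialogue array, trimming the last line after the first conversation so the gift message doesn't repeat.
; HandOnMagic adds each item to the inventory and raises magic level by item type.
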(event `self.ReceiveBeginPlay`
  ;[1 1 1] Guarda la longitud del texto (cuántas frases). Esto es útil porque, una vez que la criatura nos da la llave/magia, se resta uno a la longitud, para que no diga la frase de "ten un objeto de magia"
  (set `self.TextLenght` (`KismetArrayLibrary.Array_Length` (`self.Text`))))

(event `self.CollisionDistance.OnComponentBeginOverlap`
  (params (OverlappedComponent :type "PrimitiveComponent Object Reference") (OtherActor :type "Actor Object Reference") (OtherComp :type "PrimitiveComponent Object Reference") (OtherBodyIndex :type Integer) (bFromSweep :type Boolean) (SweepResult :type "HitResult Structure (by ref)"))
  ;[1 1 1] Cuando el personaje top-down colisiona con la caja de la criatura, se activa el booleano y se muestra el widget de presionar S para hablar
  (cast `/Game/TopDownBP/Blueprints/TopDownCharacter` OtherActor)
  (bind _astest_game_instance (cast `/Game/Blueprints/TestGameInstance` (`GameplayStatics.GetGameInstance`)))
  (set `/Game/Blueprints/TestGameInstance.OverlappingMagic` true _astest_game_instance)
  (set `/Game/Blueprints/TestGameInstance.MagicCriatureReference` self _astest_game_instance)
  (bind _pressswidget (`/Game/Blueprints/TestGameInstance.pressSwidget` _astest_game_instance))
  (if (`Widget.IsInViewport` _pressswidget)
    (`Widget.SetVisibility` _pressswidget "Visible")
    (else
      (`UserWidget.AddToViewport` _pressswidget 0))))

(event `self.CollisionDistance.OnComponentEndOverlap`
  (params (OverlappedComponent :type "PrimitiveComponent Object Reference") (OtherActor :type "Actor Object Reference") (OtherComp :type "PrimitiveComponent Object Reference") (OtherBodyIndex :type Integer))
  ;[1 1 1] Cuando se acaba el solapamiento del personaje con la caja, se desactiva el booleano y se quita el widget de presionar S y también el del dialogbox.
  (cast `/Game/TopDownBP/Blueprints/TopDownCharacter` OtherActor)
  (bind _astest_game_instance (cast `/Game/Blueprints/TestGameInstance` (`GameplayStatics.GetGameInstance`)))
  (set `/Game/Blueprints/TestGameInstance.OverlappingMagic` false _astest_game_instance)
  (`Widget.RemoveFromParent` (`/Game/Blueprints/TestGameInstance.DialogBox` _astest_game_instance))
  (`Widget.SetVisibility` (`/Game/Blueprints/TestGameInstance.pressSwidget` _astest_game_instance) "Hidden"))

(fn `getText`
  (returns (text :type Text))
  ;[1 1 1] Dado un índice, devuelve el texto en esa posición.
  (return (`|GetArrayItem` (`self.Text`) (`self.TextIndex`))))

(fn `HandOnMagic`
  ;[1 1 1] Una criatura puede tener varios ítems mágicos que dar al personaje. Este método llama a updatemagiclevel para subir la magia del personaje por cada ítem que tiene que entregarle, además, con setNItems se las añade al inventario.
  (bind _astest_game_instance (cast `/Game/Blueprints/TestGameInstance` (`GameplayStatics.GetGameInstance`)))
  (for _array_element (`self.Items`)
    (`/Game/Blueprints/TestGameInstance.SetNItems` _astest_game_instance _array_element)
    (`/Game/Blueprints/TestGameInstance.UpdateMagicLevel` _astest_game_instance (select `/Game/Blueprints/Enums/EItemType` _array_element :`NewEnumerator0` (`/Game/Blueprints/TestGameInstance.LightningValue` _astest_game_instance) :`NewEnumerator1` (`/Game/Blueprints/TestGameInstance.FlameValue` _astest_game_instance) :`NewEnumerator2` (`/Game/Blueprints/TestGameInstance.IceValue` _astest_game_instance)))
    (set `self.Spawned` true)))

(fn `nextText`
  (returns (more :type Boolean))
  (bind _textindex (`self.TextIndex`))
  ;[1 1 1] Aumenta en uno el índice por el que se va leyendo (TextIndex) si es que existe más texto, se devuelve un booleano que indica si hay más texto por mostrar o no
  (`/Engine/EditorBlueprintResources/StandardMacros.IncrementInt` _textindex
    (:`  `
      (if (< _textindex (`self.TextLenght`))
        (return true)
        (else
          (return false))))))

(fn `reloadText`
  ;[1 1 1] Recarga el texto (pone el índice a 0). Además, si es la primera vez que se habla con la criatura, se acorta en 1 la longitud del texto para que no vuelva a mostrar el mensaje de "te doy este objeto..."
  (set `self.TextIndex` 0)
  (if (`self.firstTime`)
    (`/Engine/EditorBlueprintResources/StandardMacros.DecrementInt` (`self.TextLenght`)
      (:`  `
        (set `self.firstTime` false)))))

(fn `UserConstructionScript`)