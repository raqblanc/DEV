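; AI controller for an enemy that runs the BT_Enemigo behavior tree on possession and tracks the player through AI perception.
; Sensing an actor tagged Player cancels the loss timer and writes the target and line-of-sight flag to the Blackboard.
; Any other perception update starts a timer lasting LineaDeVision, which clears both keys on expiry, giving the enemy a short memory of the player.
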(event `self.ReceivePossess`
  (params (PossessedPawn :type "Pawn Object Reference"))
  (`self.RunBehaviorTree` "/Game/Blueprints/IA/BT_Enemigo.BT_Enemigo"))

(event `self.AIPerception.OnTargetPerceptionUpdated`
  (params (Actor :type "Actor Object Reference") (Stimulus :type "AIStimulus Structure"))
  (bind _blackboard (`self.Blackboard`))
  (if (and (`.bSuccessfullySensed` (break `AIStimulus` Stimulus)) (`self.ActorHasTag` Actor "Player"))
    (`KismetSystemLibrary.K2_ClearAndInvalidateTimerHandle` (`self.TimerEnemigo`))
    (`BlackboardComponent.SetValueAsBool` _blackboard (`self.TieneLineaVision`) true)
    (`BlackboardComponent.SetValueAsObject` _blackboard (`self.ActorEnemigo`) Actor)
    (else
      (bind _returnvalue (`KismetSystemLibrary.K2_SetTimerDelegate` (delegate `StartEnemyTimer`) (`self.LineaDeVision`)))
      (set `self.TimerEnemigo` _returnvalue))))

(event `StartEnemyTimer`
  (bind _blackboard (`self.Blackboard`))
  (`BlackboardComponent.SetValueAsBool` _blackboard (`self.TieneLineaVision`) false)
  (`BlackboardComponent.SetValueAsObject` _blackboard (`self.ActorEnemigo`) null))

(fn `UserConstructionScript`)