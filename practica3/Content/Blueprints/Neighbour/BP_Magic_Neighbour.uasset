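; Magic neighbour NPC that shows a talk prompt when the player enters its collision box and registers itself with the game instance.
; It steps through a dialogue text array, switches between talking and crouched walking, and updates the game instance's magic levels from its item list.
; A helper computes spawn transforms from random navmesh points, offset by the box extent and raised above the floor, intended to keep items out of immediate reach.
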(event `self.ReceiveBeginPlay`
  (set `self.TextLenght` (`KismetArrayLibrary.Array_Length` (`self.Text`))))

(event `self.CollisionDistance.OnComponentBeginOverlap`
  (params (OverlappedComponent :type "PrimitiveComponent Object Reference") (OtherActor :type "Actor Object Reference") (OtherComp :type "PrimitiveComponent Object Reference") (OtherBodyIndex :type Integer) (bFromSweep :type Boolean) (SweepResult :type "HitResult Structure (by ref)"))
  ;[1 1 1] Cuando entra en el radio del vecino, aparece el mensaje de pulsar S para hablar
  (cast `/Game/TopDownBP/Blueprints/TopDownCharacter` OtherActor)
  (bind _astest_game_instance (cast `/Game/Blueprints/TestGameInstance` (`GameplayStatics.GetGameInstance`)))
  (set `/Game/Blueprints/TestGameInstance.OverlappingMagic` true _astest_game_instance)
  (set `/Game/Blueprints/TestGameInstance.MagicNeighbourReference` self _astest_game_instance)
  (bind _pressswidget (`/Game/Blueprints/TestGameInstance.pressSwidget` _astest_game_instance))
  (if (`Widget.IsInViewport` _pressswidget)
    (`Widget.SetVisibility` _pressswidget "Visible")
    (else
      (`UserWidget.AddToViewport` _pressswidget 0))))

(event `self.CollisionDistance.OnComponentEndOverlap`
  (params (OverlappedComponent :type "PrimitiveComponent Object Reference") (OtherActor :type "Actor Object Reference") (OtherComp :type "PrimitiveComponent Object Reference") (OtherBodyIndex :type Integer))
  ;[1 1 1] Cuando entra en el radio del vecino, aparece el mensaje de pulsar S para hablar
  (cast `/Game/TopDownBP/Blueprints/TopDownCharacter` OtherActor)
  (bind _astest_game_instance (cast `/Game/Blueprints/TestGameInstance` (`GameplayStatics.GetGameInstance`)))
  (set `/Game/Blueprints/TestGameInstance.OverlappingMagic` false _astest_game_instance)
  (`Widget.RemoveFromParent` (`/Game/Blueprints/TestGameInstance.DialogBox` _astest_game_instance)))

(fn `calculatePoint`
  (params (CollisionPoint :type "Float (double-precision)") (RandomPoint :type "Float (double-precision)"))
  (returns (SpawnPoint :type "Float (double-precision)"))
  ;[1 1 1] Collision point es el tamaño de la caja de colisión. Esta función calcula un punto que salga fuera de la caja (para que no haya posibilidad de que el player coja el objeto sin tener que desplazarse). Vale para X y para Y.
  (if (< RandomPoint 0.0)
    (return (- RandomPoint CollisionPoint))
    (else
      (return (+ CollisionPoint RandomPoint)))))

(fn `getSpawnTransform`
  (returns (transform :type "Transform Structure"))
  (locals (X :type "Float (double-precision)" :default 0.0) (Y :type "Float (double-precision)"))
  (bind _spawnpoint (`self.calculatePoint` (.x (`BoxComponent.GetScaledBoxExtent` (`self.CollisionDistance`))) (.x (`NavigationSystemV1.K2_GetRandomLocationInNavigableRadius` (.location (`self.GetTransform`)) 500.0 null "/Script/NavigationSystem.RecastFilter_UseDefaultArea"))))
  (bind _output_get (set `local.X` _spawnpoint))
  (bind _spawnpoint_2 (`self.calculatePoint` (.y (`BoxComponent.GetScaledBoxExtent` (`self.CollisionDistance`))) (.y (`NavigationSystemV1.K2_GetRandomLocationInNavigableRadius` (.location (`self.GetTransform`)) 500.0 null "/Script/NavigationSystem.RecastFilter_UseDefaultArea"))))
  (bind _output_get_2 (set `local.Y` _spawnpoint_2))
  (return (`KismetMathLibrary.MakeTransform` (`KismetMathLibrary.MakeVector` _output_get _output_get_2 (+ (.z (`NavigationSystemV1.K2_GetRandomLocationInNavigableRadius` (.location (`self.GetTransform`)) 500.0 null "/Script/NavigationSystem.RecastFilter_UseDefaultArea")) 50.0)) (.rotation (`self.GetTransform`)) (.scale (`self.GetTransform`)))))

(fn `getText`
  (returns (text :type Text))
  (return (`|GetArrayItem` (`self.Text`) (`self.TextIndex`))))

(fn `HandOnMagic`
  (bind _astest_game_instance (cast `/Game/Blueprints/TestGameInstance` (`GameplayStatics.GetGameInstance`)))
  (for _array_element (`self.Items`)
    (`/Game/Blueprints/TestGameInstance.UpdateMagicLevel` _astest_game_instance (select `/Game/Blueprints/EItemType` _array_element :`NewEnumerator0` (`/Game/Blueprints/TestGameInstance.LightningValue` _astest_game_instance) :`NewEnumerator1` (`/Game/Blueprints/TestGameInstance.FlameValue` _astest_game_instance) :`NewEnumerator2` (`/Game/Blueprints/TestGameInstance.SnowFlakeValue` _astest_game_instance)))
    (set `self.Spawned` true)))

(fn `nextText`
  (returns (more :type Boolean))
  (bind _textindex (`self.TextIndex`))
  (`/Engine/EditorBlueprintResources/StandardMacros.IncrementInt` _textindex
    (:`  `
      (if (< _textindex (`self.TextLenght`))
        (return true)
        (else
          (return false))))))

(fn `reloadText`
  (params (magicOK :type Boolean))
  (if (not magicOK)
    (`/Engine/EditorBlueprintResources/StandardMacros.DecrementInt` (`self.TextLenght`)
      (:`  `
        _)))
  (set `self.TextIndex` 0))

(fn `Speak`
  (bind _astest_game_instance (cast `/Game/Blueprints/TestGameInstance` (`GameplayStatics.GetGameInstance`)))
  (if (`/Game/Blueprints/TestGameInstance.OverlappingKey` _astest_game_instance)
    _))

(fn `StartNeighbour`
  (set `CharacterMovementComponent.MaxWalkSpeed` 100.0 (`self.CharacterMovement`))
  (`SkeletalMeshComponent.PlayAnimation` (`self.Mesh`) "/Game/Downloaded/Mixiamo/Crouched_Walking_Anim_mixamo_com.Crouched_Walking_Anim_mixamo_com" true))

(fn `StopNeighbour`
  (set `CharacterMovementComponent.MaxWalkSpeed` 0.0 (`self.CharacterMovement`))
  (`SkeletalMeshComponent.PlayAnimation` (`self.Mesh`) "/Game/Downloaded/Mixiamo/Talking_Anim_mixamo_com.Talking_Anim_mixamo_com" true))

(fn `UserConstructionScript`)