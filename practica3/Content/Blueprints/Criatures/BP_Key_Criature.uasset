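; Talking creature NPC that gives the player a magic sphere key (BP_Key) once.
; Box overlap with the TopDownCharacter registers the creature in TestGameInstance and toggles the press-S and dialog widgets.
; Exposed functions halt or resume walking with animation swaps, page through the Text array, and spawn the KeyType-materialed key at a nearby random navigable point.
; ReloadText rewinds dialogue, trimming the final gift line while the key is unspawned.
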(event `self.ReceiveBeginPlay`
  ;[1 1 1] Recarga el texto (pone el índice a 0). Además, si es la primera vez que se habla con la criatura, se acorta en 1 la longitud del texto para que no vuelva a mostrar el mensaje de "te doy este objeto..."
  (set `self.textLenght` (`KismetArrayLibrary.Array_Length` (`self.Text`))))

(event `self.CollisionDistance.OnComponentBeginOverlap`
  (params (OverlappedComponent :type "PrimitiveComponent Object Reference") (OtherActor :type "Actor Object Reference") (OtherComp :type "PrimitiveComponent Object Reference") (OtherBodyIndex :type Integer) (bFromSweep :type Boolean) (SweepResult :type "HitResult Structure (by ref)"))
  ;[1 1 1] Cuando el personaje top-down colisiona con la caja de la criatura, se activa el booleano y se muestra el widget de presionar S para hablar
  (cast `/Game/TopDownBP/Blueprints/TopDownCharacter` OtherActor)
  (bind _astest_game_instance (cast `/Game/Blueprints/TestGameInstance` (`GameplayStatics.GetGameInstance`)))
  (set `/Game/Blueprints/TestGameInstance.KeyCriatureReference` self _astest_game_instance)
  (set `/Game/Blueprints/TestGameInstance.OverlappingKey` true _astest_game_instance)
  (bind _pressswidget (`/Game/Blueprints/TestGameInstance.pressSwidget` _astest_game_instance))
  (if (`Widget.IsInViewport` _pressswidget)
    (`Widget.SetVisibility` _pressswidget "Visible")
    (else
      (`UserWidget.AddToViewport` _pressswidget 0))))

(event `self.CollisionDistance.OnComponentEndOverlap`
  (params (OverlappedComponent :type "PrimitiveComponent Object Reference") (OtherActor :type "Actor Object Reference") (OtherComp :type "PrimitiveComponent Object Reference") (OtherBodyIndex :type Integer))
  ;[1 1 1] Cuando se acaba el solapamiento del personaje con la caja, se desactiva el booleano y se quita el widget de presionar S y también el del dialogbox.
  (cast `/Game/TopDownBP/Blueprints/TopDownCharacter` OtherActor)
  (bind _astest_game_instance (cast `/Game/Blueprints/TestGameInstance` (`GameplayStatics.GetGameInstance`)))
  (set `/Game/Blueprints/TestGameInstance.OverlappingKey` false _astest_game_instance)
  (`Widget.RemoveFromParent` (`/Game/Blueprints/TestGameInstance.DialogBox` _astest_game_instance))
  (`Widget.SetVisibility` (`/Game/Blueprints/TestGameInstance.pressSwidget` _astest_game_instance) "Hidden"))

(fn `getSpawnTransform`
  (returns (transform :type "Transform Structure"))
  (locals (X :type "Float (double-precision)" :default 0.0) (Y :type "Float (double-precision)"))
  ;[1 1 1] Devuelve una transformación generada aleatoriamente donde spawnear la esferam mágica (llave)
  (return (`KismetMathLibrary.MakeTransform` (`KismetMathLibrary.MakeVector` (.x (`NavigationSystemV1.K2_GetRandomLocationInNavigableRadius` (.location (`self.GetTransform`)) 300.0 null "/Script/NavigationSystem.RecastFilter_UseDefaultArea")) (.y (`NavigationSystemV1.K2_GetRandomLocationInNavigableRadius` (.location (`self.GetTransform`)) 300.0 null "/Script/NavigationSystem.RecastFilter_UseDefaultArea")) (+ (.z (`NavigationSystemV1.K2_GetRandomLocationInNavigableRadius` (.location (`self.GetTransform`)) 300.0 null "/Script/NavigationSystem.RecastFilter_UseDefaultArea")) 50.0)) (.rotation (`self.GetTransform`)) (.scale (`self.GetTransform`)))))

(fn `getText`
  (returns (text :type Text))
  ;[1 1 1] Dado un índice, devuelve el texto en esa posición.
  (return (`|GetArrayItem` (`self.Text`) (`self.TextIndex`))))

(fn `nextText`
  (returns (more :type Boolean))
  (bind _textindex (`self.TextIndex`))
  ;[1 1 1] Aumenta en uno el índice por el que se va leyendo (TextIndex) si es que existe más texto, se devuelve un booleano que indica si hay más texto por mostrar o no
  (`/Engine/EditorBlueprintResources/StandardMacros.IncrementInt` _textindex
    (:`  `
      (if (< _textindex (`self.TextLenght`))
        (return true)
        (else
          (return false))))))

(fn `ReloadText`
  ;[1 1 1] Recarga el texto (pone el índice a 0). Además, si es la primera vez que se habla con la criatura, se acorta en 1 la longitud del texto para que no vuelva a mostrar el mensaje de "te doy este objeto..."
  (if (not (`self.Spawned`))
    (`/Engine/EditorBlueprintResources/StandardMacros.DecrementInt` (`self.textLenght`)
      (:`  `
        _)))
  (set `self.TextIndex` 0))

(fn `SpawnKey`
  ;[1 1 1] Spawnea la esfera mágica (llave) si no se había ya spawneado y si se está haciendo overlap con la criatura.
  (bind _astest_game_instance (cast `/Game/Blueprints/TestGameInstance` (`GameplayStatics.GetGameInstance`)))
  (if (and (not (`self.Spawned`)) (`/Game/Blueprints/TestGameInstance.OverlappingKey` _astest_game_instance))
    (set `self.Spawned` true)
    (bind _transform (`self.getSpawnTransform`))
    (bind _returnvalue (`|SpawnActorFromClass` "/Game/Blueprints/Objects/BP_Key.BP_Key_C" _transform "AdjustIfPossibleButAlwaysSpawn" "OverrideRootScale" null null))
    (`/Game/Blueprints/Objects/BP_Key.setMaterial` _returnvalue (`self.KeyType`))))

(fn `Speak`
  ;[1 1 1] Desactiva el widget de presionar S para hablar, porque ya están hablando
  (bind _astest_game_instance (cast `/Game/Blueprints/TestGameInstance` (`GameplayStatics.GetGameInstance`)))
  (if (`/Game/Blueprints/TestGameInstance.OverlappingKey` _astest_game_instance)
    (`Widget.SetVisibility` (`/Game/Blueprints/TestGameInstance.pressSwidget` _astest_game_instance) "Hidden")))

(fn `Start`
  ;[1 1 1] La criatura reanuda su marcha (velocidad 100) y se activa la animación walking
  (set `CharacterMovementComponent.MaxWalkSpeed` 100.0 (`self.CharacterMovement`))
  (`SkeletalMeshComponent.PlayAnimation` (`self.Mesh`) "/Game/Mixiamo/Crouched_Walking_Anim_mixamo_com.Crouched_Walking_Anim_mixamo_com" true))

(fn `Stop`
  ;[1 1 1] Para a la criatura (velocidad a 0) y se activa la animación talking
  (set `CharacterMovementComponent.MaxWalkSpeed` 0.0 (`self.CharacterMovement`))
  (`SkeletalMeshComponent.PlayAnimation` (`self.Mesh`) "/Game/Mixiamo/Talking_Anim_mixamo_com.Talking_Anim_mixamo_com" true))

(fn `UserConstructionScript`)