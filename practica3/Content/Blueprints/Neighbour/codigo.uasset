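; Neighbour actor that shows a press-S prompt when the player character comes near and spawns a key on interaction.
; Box overlap events track proximity and toggle a shared prompt widget held by TestGameInstance.
; Pressing S while overlapping hides the prompt and, only the first time, spawns a BP_Key at a random navigable point nearby, slightly raised, with its material set from KeyType.
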(event `self.ReceiveBeginPlay`
  ;[1 1 1] Cuando entra en el radio del vecino, aparece el mensaje de pulsar S para hablar
  (`self.EnableInput` (`GameplayStatics.GetPlayerController` 0)))

(event `Key|S`
  (params (Key :type "Key Structure"))
  (:`Pressed`
    (if (`self.Overlapping`)
      (`Widget.SetVisibility` (`/Game/Blueprints/TestGameInstance.pressSwidget` (stale `self.Box.OnComponentBeginOverlap` _astest_game_instance)) "Hidden")
      (if (not (`self.Spawned`))
        ;[1 1 1] Spawnea al objeto llave
        (set `self.Spawned` true)
        (bind _returnvalue (`|SpawnActorFromClass` "/Game/Blueprints/BP_Key.BP_Key_C" (`KismetMathLibrary.MakeTransform` (`KismetMathLibrary.MakeVector` (.x (`NavigationSystemV1.K2_GetRandomLocationInNavigableRadius` (.location (`self.GetTransform`)) 200.0 null "/Script/NavigationSystem.RecastFilter_UseDefaultArea")) (.y (`NavigationSystemV1.K2_GetRandomLocationInNavigableRadius` (.location (`self.GetTransform`)) 200.0 null "/Script/NavigationSystem.RecastFilter_UseDefaultArea")) (+ (.z (`NavigationSystemV1.K2_GetRandomLocationInNavigableRadius` (.location (`self.GetTransform`)) 200.0 null "/Script/NavigationSystem.RecastFilter_UseDefaultArea")) 50.0)) (.rotation (`self.GetTransform`)) (.scale (`self.GetTransform`))) "AdjustIfPossibleButAlwaysSpawn" "OverrideRootScale" null null))
        (`/Game/Blueprints/BP_Key.setMaterial` _returnvalue (`self.KeyType`))))))

(event `self.Box.OnComponentBeginOverlap`
  (params (OverlappedComponent :type "PrimitiveComponent Object Reference") (OtherActor :type "Actor Object Reference") (OtherComp :type "PrimitiveComponent Object Reference") (OtherBodyIndex :type Integer) (bFromSweep :type Boolean) (SweepResult :type "HitResult Structure (by ref)"))
  ;[1 1 1] Cuando entra en el radio del vecino, aparece el mensaje de pulsar S para hablar
  (set `self.Overlapping` true)
  (cast `/Game/TopDownBP/Blueprints/TopDownCharacter` OtherActor)
  (bind _astest_game_instance (cast `/Game/Blueprints/TestGameInstance` (`GameplayStatics.GetGameInstance`)))
  (bind _pressswidget (`/Game/Blueprints/TestGameInstance.pressSwidget` _astest_game_instance))
  (if (`Widget.IsInViewport` _pressswidget)
    (`Widget.SetVisibility` _pressswidget "Visible")
    (else
      (`UserWidget.AddToViewport` _pressswidget 0))))

(event `self.Box.OnComponentEndOverlap`
  (params (OverlappedComponent :type "PrimitiveComponent Object Reference") (OtherActor :type "Actor Object Reference") (OtherComp :type "PrimitiveComponent Object Reference") (OtherBodyIndex :type Integer))
  ;[1 1 1] Cuando entra en el radio del vecino, aparece el mensaje de pulsar S para hablar
  (cast `/Game/TopDownBP/Blueprints/TopDownCharacter` OtherActor)
  (set `self.Overlapping` false)
  (`Widget.SetVisibility` (`/Game/Blueprints/TestGameInstance.pressSwidget` (stale `self.Box.OnComponentBeginOverlap` _astest_game_instance)) "Hidden"))

(fn `UserConstructionScript`)