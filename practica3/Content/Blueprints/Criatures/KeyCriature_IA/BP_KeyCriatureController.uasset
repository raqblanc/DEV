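; AI controller for the KeyCriature, a creature the player can talk with.
; On possess it runs the BT_KeyCriature behavior tree.
; StillTalking sets the Talk and Continue blackboard keys to keep the conversation going, and StopTalking clears Continue to end it, leaving Talk untouched.
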(event `self.ReceivePossess`
  (params (PossessedPawn :type "Pawn Object Reference"))
  (`self.RunBehaviorTree` "/Game/Blueprints/Criatures/KeyCriature_IA/BT_KeyCriature.BT_KeyCriature"))

(fn `StillTalking`
  (bind _blackboard (`self.Blackboard`))
  ;[1 1 1] Activa talk y continue para seguir hablando con el personaje
  (`BlackboardComponent.SetValueAsBool` _blackboard (`self.Talk`) true)
  (`BlackboardComponent.SetValueAsBool` _blackboard (`self.Continue`) true))

(fn `Stop Talking`
  ;[1 1 1] Desactiva continue para dejar de hablar
  (`BlackboardComponent.SetValueAsBool` (`self.Blackboard`) (`self.Continue`) false))

(fn `UserConstructionScript`)