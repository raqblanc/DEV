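; BP_LevelTransition is a level portal that lets the player character travel to another level when its key and magic requirements are met.
; On overlap, it checks the GameInstance for exactly one key of the required type and enough magic, then plays a teleport sound and opens the level after a short delay.
; Otherwise it shows the GameInstance's portal widget until overlap ends.
; The construction script derives required magic from key type.
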(event `self.ReceiveBeginPlay`
  ;[1 1 1] Guarda una referencia a gameinstance al comienzo
  (bind _astest_game_instance (cast `/Game/Blueprints/TestGameInstance` (`GameplayStatics.GetGameInstance`)))
  (set `self.GameInstance` _astest_game_instance))

(event `self.Overlap.OnComponentBeginOverlap`
  (params (OverlappedComponent :type "PrimitiveComponent Object Reference") (OtherActor :type "Actor Object Reference") (OtherComp :type "PrimitiveComponent Object Reference") (OtherBodyIndex :type Integer) (bFromSweep :type Boolean) (SweepResult :type "HitResult Structure (by ref)"))
  (bind _gameinstance (`self.GameInstance`))
  (bind _portalwidgetreference (`/Game/Blueprints/TestGameInstance.PortalWidgetReference` (`self.GameInstance`)))
  ;[1 1 1] Si se hace overlap con la caja del portal, se verifica la condición de que haya una orbe (llave) del tipo de nivel y que la magia del personaje sea >= que la requerida, se reproduce el sonido de portal y se abre el siguiente nivel. Si no se cumple, se muestra el widget que indica que no se puede cruzar el portal
  (cast `/Game/TopDownBP/Blueprints/TopDownCharacter` OtherActor)
  (bind _value (`/Game/Blueprints/TestGameInstance.GetNKeys` _gameinstance (`self.RequireKeyType`)))
  (if (and (== _value 1) (<= (`self.required_magic_level`) (`/Game/Blueprints/TestGameInstance.MagicLevel` _gameinstance)))
    (`GameplayStatics.PlaySoundAtLocation` "/Game/TandP/Sound_Effects/S_Teleport.S_Teleport" (`self.K2_GetActorLocation`) (struct) 1.0 1.0 0.0 null null null)
    (`KismetSystemLibrary.Delay` 1.0) ; Sirve para que al menos se oiga 1 segundo del audio que se reproduce
    (`GameplayStatics.OpenLevel` (`self.LevelName`))
    (elif (`Widget.IsInViewport` _portalwidgetreference)
      (`Widget.SetVisibility` _portalwidgetreference "Visible")
      (else
        (`UserWidget.AddToViewport` _portalwidgetreference 0)))))

(event `self.Overlap.OnComponentEndOverlap`
  (params (OverlappedComponent :type "PrimitiveComponent Object Reference") (OtherActor :type "Actor Object Reference") (OtherComp :type "PrimitiveComponent Object Reference") (OtherBodyIndex :type Integer))
  ;[1 1 1] Cuando se deja de hacer overlap, se desactiva el widget del portal
  (cast `/Game/TopDownBP/Blueprints/TopDownCharacter` OtherActor)
  (`Widget.SetVisibility` (`/Game/Blueprints/TestGameInstance.PortalWidgetReference` (`self.GameInstance`)) "Hidden"))

(fn `UserConstructionScript`
  ;[1 1 1] Se establece el valor de nivel de magia requerido para el portal dependiendo del tipo de llave que se requiere
  (set `self.required_magic_level` (select `/Game/Blueprints/Enums/EKeyType` (`self.RequireKeyType`) :`NewEnumerator1` (`self.FireWorld`) :`NewEnumerator2` (`self.LightningWorld`) :`NewEnumerator3` (`self.IceWorld`))))