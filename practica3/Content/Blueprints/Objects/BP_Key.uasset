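; BP_Key is a magic orb pickup that acts as a fire, lightning or ice world key.
; The construction script sets the orb's material from KeyType via SetMaterial, which also stores the type passed in.
; When TopDownCharacter overlaps it, the orb waits briefly, registers the key through TestGameInstance's SetNKeys and destroys itself.
; The delay works around overlaps firing before the key type is set.
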(event `self.ReceiveBeginPlay`
  (bind _astest_game_instance (cast `/Game/Blueprints/TestGameInstance` (`GameplayStatics.GetGameInstance`)))
  (set `self.GameInstance` _astest_game_instance))

(event `self.Overlap.OnComponentBeginOverlap`
  (params (OverlappedComponent :type "PrimitiveComponent Object Reference") (OtherActor :type "Actor Object Reference") (OtherComp :type "PrimitiveComponent Object Reference") (OtherBodyIndex :type Integer) (bFromSweep :type Boolean) (SweepResult :type "HitResult Structure (by ref)"))
  ;[1 1 1] Cuando se hace overlap con el orbe mágico (llave) se espera 1 segundo, se añade la llave al inventario del personaje y se destruye el orbe
  (cast `/Game/TopDownBP/Blueprints/TopDownCharacter` OtherActor)
  (`KismetSystemLibrary.Delay` 1.0) ; Esta espera es necesaria porque, si no se hace, el personaje puede hacer overlap con el orbe antes de que se haga el "set material" del orbe (donde se añade el tipo de llave), generando un error.
  (`/Game/Blueprints/TestGameInstance.SetNKeys` (`self.GameInstance`) (`self.KeyType`))
  (`self.K2_DestroyActor`))

(fn `setMaterial`
  (params (Type :type "/Game/Blueprints/Enums/EKeyType Enum" :default "NewEnumerator1"))
  ;[1 1 1] Cambia el material del orbe dependiendo de de qué tipo es
  (bind _output_get (set `self.KeyType` Type))
  (`PrimitiveComponent.SetMaterial` (`self.Key`) 0 (select `/Game/Blueprints/Enums/EKeyType` _output_get :`NewEnumerator1` "/Game/Materials/M_FireKey.M_FireKey" :`NewEnumerator2` "/Game/Materials/M_LightningKey.M_LightningKey" :`NewEnumerator3` "/Game/Materials/M_IceKey.M_IceKey" :!type "MaterialInterface Object Reference")))

(fn `UserConstructionScript`
  (`self.setMaterial` (`self.KeyType`)))