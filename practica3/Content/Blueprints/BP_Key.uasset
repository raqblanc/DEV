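; BP_Key is a collectible key pickup for a top-down game, typed by area such as Basement, FirstFloor or SecondFloor.
; The construction script picks the key mesh's colored material from its KeyType, so each variant shows its color in the editor.
; When a TopDownCharacter overlaps it, the key adds its type to that character's OwnedKeys, calls SetNKeys for that type and destroys itself.
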(event `self.Overlap.OnComponentBeginOverlap`
  (params (OverlappedComponent :type "PrimitiveComponent Object Reference") (OtherActor :type "Actor Object Reference") (OtherComp :type "PrimitiveComponent Object Reference") (OtherBodyIndex :type Integer) (bFromSweep :type Boolean) (SweepResult :type "HitResult Structure (by ref)"))
  (bind _keytype (`self.KeyType`))
  (bind _astop_down_character (cast `/Game/TopDownBP/Blueprints/TopDownCharacter` OtherActor))
  (`KismetArrayLibrary.Array_Add` (`/Game/TopDownBP/Blueprints/TopDownCharacter.OwnedKeys` _astop_down_character) _keytype)
  (`/Game/TopDownBP/Blueprints/TopDownCharacter.set_n_keys` _astop_down_character _keytype)
  (`self.K2_DestroyActor`))

(fn `UserConstructionScript`
  (`PrimitiveComponent.SetMaterial` (`self.Key`) 0 (select `/Game/Blueprints/EKeyType` (`self.KeyType`) :`NewEnumerator0` "/Game/Blueprints/M_Key.M_Key" :`NewEnumerator1` "/Game/Blueprints/M_BlueKey.M_BlueKey" :`NewEnumerator2` "/Game/Blueprints/M_RedKey.M_RedKey" :`NewEnumerator3` "/Game/Blueprints/M_GreenKey.M_GreenKey" :!type "MaterialInterface Object Reference")))